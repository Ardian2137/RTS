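; Base RTS-style unit that sets its material by team, registers player units with the camera pawn's selection component, and shows a cursor when selected.
; On BeginPlay it spawns its controller and hand and forearm weapons, and binds health and mana changes to a statistics bar widget.
; Tick rotates the bars using camera height and turns the unit toward its attack target.
; Overlap-based enemy detection and targeting logic is disconnected.
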(event `self.HandleSelection`
  (params (bSelected :type Boolean))
  (`SceneComponent.SetHiddenInGame` (`self.CursorToWorld`) (not bSelected) false))

(event `self.ReceiveBeginPlay`
  (`|ExecutionSequence`
    (:`then_0`
      (`self.SpawnDefaultController`)
      (switch `ETeam` (`self.Team`)
        (:`Player`
          (`PrimitiveComponent.SetMaterial` (`self.Mesh`) 0 "/Game/StarterContent/Materials/M_Water_Lake.M_Water_Lake")
          (`KismetArrayLibrary.Array_Add` (`UnitsSelectionComponent.AllControlledUnits` (`PlayerCameraPawn.UnitsSelectionComponent` (`/Game/MainContent/GameBPs/BP_GlobalFunctions.GetPlayerCameraPawn`))) self))
        (:`AI`
          (`PrimitiveComponent.SetMaterial` (`self.Mesh`) 0 "/Game/AnimStarterPack/UE4_Mannequin/Materials/M_UE4Man_Body.M_UE4Man_Body"))
        (:`Unknown`
          (`PrimitiveComponent.SetMaterial` (`self.Mesh`) 0 "/Game/StarterContent/Materials/M_Wood_Pine.M_Wood_Pine"))))
    (:`then_1`
      (add `HealthComponent.OnHealthAmountChanged` (`self.HealthComponent`) (delegate `OnHealthAmountChanged`))
      (add `ManaComponent.OnManaAmountChanged` (`self.ManaComponent`) (delegate `OnManaAmountChanged`)))
    (:`then_2`
      (`|ExecutionSequence`
        (:`then_0`
          (bind _returnvalue (`|SpawnActorFromClass` (`WeaponComponent.RightWeaponClass` (`self.WeaponComponent`)) (`KismetMathLibrary.MakeTransform` (0.0 0.0 0.0)) "Undefined" "OverrideRootScale" null null))
          (`self.K2_AttachToComponent` _returnvalue (`self.Mesh`) "RightHand" "KeepRelative" "KeepRelative" "KeepRelative" true)
          (set `WeaponComponent.RightWeapon` _returnvalue (`self.WeaponComponent`)))
        (:`then_1`
          (bind _returnvalue_2 (`|SpawnActorFromClass` (`WeaponComponent.LeftWeaponClass` (`self.WeaponComponent`)) (`KismetMathLibrary.MakeTransform` (0.0 0.0 0.0)) "Undefined" "OverrideRootScale" null null))
          (`self.K2_AttachToComponent` _returnvalue_2 (`self.Mesh`) "LeftForarm" "KeepRelative" "KeepRelative" "KeepRelative" true)
          (set `WeaponComponent.LeftWeapon` _returnvalue_2 (`self.WeaponComponent`)))))))

(event `OnHealthAmountChanged`
  (bind _aswb_statistics_bars (cast `/Game/MainContent/UI/WB_StatisticsBars` (`WidgetComponent.GetUserWidgetObject` (`self.StatisticsBars`))))
  (`/Game/MainContent/UI/WB_StatisticsBars.SetHealthPercent` _aswb_statistics_bars (`HealthComponent.GetHealthPercentage` (`self.HealthComponent`))))

(event `OnManaAmountChanged`
  (bind _aswb_statistics_bars (cast `/Game/MainContent/UI/WB_StatisticsBars` (`WidgetComponent.GetUserWidgetObject` (`self.StatisticsBars`))))
  (`/Game/MainContent/UI/WB_StatisticsBars.SetManaPercent` _aswb_statistics_bars (`ManaComponent.GetManaPercentage` (`self.ManaComponent`))))

(event `self.ReceiveTick`
  (params (DeltaSeconds :type "Float (single-precision)"))
  ;[1 1 1] event tick
  (`|ExecutionSequence`
    (:`then_0`
      (`SceneComponent.K2_SetWorldRotation` (`self.StatisticsBars`) (`KismetMathLibrary.FindLookAtRotation` (`KismetMathLibrary.MakeVector` 0.0 0.0 (.z (`SceneComponent.K2_GetComponentLocation` (`self.StatisticsBars`)))) (`KismetMathLibrary.MakeVector` 0.0 0.0 (.z (`PlayerCameraManager.GetCameraLocation` (`GameplayStatics.GetPlayerCameraManager` 0))))) false false))
    (:`then_1`
      (if (`self.bHasTargetToAttack`)
        (bind _output_get (set `self.TargetRotation` (`KismetMathLibrary.FindLookAtRotation` (`self.K2_GetActorLocation`) (`self.K2_GetActorLocation` (`self.UnitTargetToAttack`)))))
        (`self.K2_SetActorRotation` _output_get)))))

(event `self.Sphere.OnComponentBeginOverlap`
  (params (OverlappedComponent :type "PrimitiveComponent Object Reference") (OtherActor :type "Actor Object Reference") (OtherComp :type "PrimitiveComponent Object Reference") (OtherBodyIndex :type Integer) (bFromSweep :type Boolean) (SweepResult :type "HitResult Structure (by ref)"))
  ;[1 1 1] on comp begin overlap
)

(event `self.Sphere.OnComponentEndOverlap`
  (params (OverlappedComponent :type "PrimitiveComponent Object Reference") (OtherActor :type "Actor Object Reference") (OtherComp :type "PrimitiveComponent Object Reference") (OtherBodyIndex :type Integer))
  ;[1 1 1] on comp end overlap
)

(fn `UserConstructionScript`)