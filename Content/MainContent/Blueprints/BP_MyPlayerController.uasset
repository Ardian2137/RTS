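; RTS player controller that drives the camera pawn and commands the player's units.
; Keys and screen-edge mouse movement move the camera at a zoom-scaled speed; zoom adjusts spring arm length, and holding pan rotates the view through gates, suspending edge movement.
; Left-drag flags a selection box, passing HUD-selected Player-team units to the pawn's selection component.
; Right-click sends selected units to the cursor hit via AI SimpleMoveToLocation, targeting AI-team units for attack.
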(event `self.ReceiveBeginPlay`
  ;[1 1 1] begin play
  (`|ExecutionSequence`
    (:`then_0`
      (`self.ReferenceCasts`))
    (:`then_1`
      (`WidgetBlueprintLibrary.SetInputMode_GameAndUIEx` self null "LockAlways" false))))

(event `InputAction|zoomIn`
  (params (Key :type "Key Structure"))
  (bind _springarm (`/Game/MainContent/Blueprints/BP_PlayerCameraPawn.SpringArm` (`self.CameraPawnRef`)))
  ;[0.1952 1 0.08493] Camera movement
  ;;[0.09543 0.1731 1] My tryin to zoom in
  (:`Pressed`
    (set `SpringArmComponent.TargetArmLength` (`KismetMathLibrary.FClamp` (- (`SpringArmComponent.TargetArmLength` _springarm) 120.0) (`self.MinZoom`) (`self.MaxZoom`)) _springarm)))

(event `InputAxis|MoveForward`
  (params (AxisValue :type "Float (single-precision)"))
  ;[0.1952 1 0.08493] Camera movement
  ;;[1 1 1] movement x
  (if (not false)
    (`self.K2_SetActorTransform` (`self.CameraPawnRef`) (`KismetMathLibrary.MakeTransform` (`KismetMathLibrary.MakeVector` (.x (.location (`self.MovementX` AxisValue (`self.MovementSpeedCalculation`) (`self.FastMoveMultiplier`) (`self.CameraPawnRef`)))) (.y (.location (`self.MovementX` AxisValue (`self.MovementSpeedCalculation`) (`self.FastMoveMultiplier`) (`self.CameraPawnRef`)))) 100.0) (.rotation (`self.MovementX` AxisValue (`self.MovementSpeedCalculation`) (`self.FastMoveMultiplier`) (`self.CameraPawnRef`))) (.scale (`self.MovementX` AxisValue (`self.MovementSpeedCalculation`) (`self.FastMoveMultiplier`) (`self.CameraPawnRef`)))) false false)))

(event `InputAction|zoomOut`
  (params (Key :type "Key Structure"))
  (bind _springarm (`/Game/MainContent/Blueprints/BP_PlayerCameraPawn.SpringArm` (`self.CameraPawnRef`)))
  ;[0.1952 1 0.08493] Camera movement
  ;;[0.1703 0.2932 1] My tryin to zoom out
  (:`Pressed`
    (set `SpringArmComponent.TargetArmLength` (`KismetMathLibrary.FClamp` (- (`SpringArmComponent.TargetArmLength` _springarm) -120.0) (`self.MinZoom`) (`self.MaxZoom`)) _springarm)))

(event `InputAxis|MoveRight`
  (params (AxisValue :type "Float (single-precision)"))
  ;[0.1952 1 0.08493] Camera movement
  ;;[1 1 1] movement z
  (if (not false)
    (`self.K2_SetActorTransform` (`self.CameraPawnRef`) (`self.MovementY` AxisValue (`self.MovementSpeedCalculation`) (`self.FastMoveMultiplier`) (`self.CameraPawnRef`)) false false)))

(event `Key|LeftMouseButton`
  (params (Key :type "Key Structure"))
  ;[1 1 1] left mouse buttton
  (:`Pressed`
    (set `self.bSelectionRecActive` true)
    (set `self.b1stPointSet` true))
  (:`Released`
    (set `self.b1stPointSet` false)
    (set `self.bSelectionRecActive` false)
    (bind _sortedcharacters (`self.SortMyCharactersByTeam` (`self.UnitsSelectedByHUD`)))
    (`UnitsSelectionComponent.SetCurrentlySelectedUnits` (`PlayerCameraPawn.UnitsSelectionComponent` (`/Game/MainContent/GameBPs/BP_GlobalFunctions.GetPlayerCameraPawn`)) _sortedcharacters)))

(event `InputAction|panReset`
  (params (Key :type "Key Structure"))
  ;[0.1952 1 0.08493] Camera movement
  ;;[1 1 1] panReset
  (:`Pressed`
    (`self.K2_SetActorRotation` (`self.CameraPawnRef`) (`KismetMathLibrary.MakeRotator` 0.0) false)))

(event `InputAxisKey|MouseX`
  (params (AxisValue :type "Float (single-precision)"))
  ;[0.1952 1 0.08493] Camera movement
  ;;[1 1 1] pan X
  (`/Engine/EditorBlueprintResources/StandardMacros.Gate` true :!label _label
    (:`Exit`
      (`self.K2_SetActorRotation` (`self.CameraPawnRef`) (`KismetMathLibrary.MakeRotator` (.roll (`self.K2_GetActorRotation` (`self.CameraPawnRef`))) (.pitch (`self.K2_GetActorRotation` (`self.CameraPawnRef`))) (+ (.yaw (`self.K2_GetActorRotation` (`self.CameraPawnRef`))) (* (`self.PanSensitivity`) AxisValue))) false))))

(event `InputAction|pan`
  (params (Key :type "Key Structure"))
  ;[0.1952 1 0.08493] Camera movement
  ;;[1 1 1] pan X
  (:`Pressed`
    (set `self.bDisableCamNav` true)
    (goto _label :!via `Open`))
  (:`Released`
    (set `self.bDisableCamNav` false)
    (goto _label :!via `Close`)))

(event `InputAction|ZoomReset`
  (params (Key :type "Key Structure"))
  ;[0.1952 1 0.08493] Camera movement
  ;;[1 1 1] Zoom reset
  (:`Pressed`
    (set `SpringArmComponent.TargetArmLength` 1500.0 (`/Game/MainContent/Blueprints/BP_PlayerCameraPawn.SpringArm` (`self.CameraPawnRef`)))))

(event `Key|RightMouseButton`
  (params (Key :type "Key Structure"))
  (bind (_bblockinghit _binitialoverlap _time _distance _location _impactpoint _normal _impactnormal _physmat _hitactor) (`GameplayStatics.BreakHitResult` (`self.GetHitResultUnderCursorByChannel` (`GameplayStatics.GetPlayerController` 0) "TraceTypeQuery1" true)))
  ;[1 1 1] Right mouse button: simple move selected actors
  (:`Pressed`
    (for _array_element (`UnitsSelectionComponent.CurrentlySelectedUnits` (`PlayerCameraPawn.UnitsSelectionComponent` (`/Game/MainContent/GameBPs/BP_GlobalFunctions.GetPlayerCameraPawn`)))
      (bind _asbp_basic_unit (cast `/Game/MainContent/Blueprints/BP_BasicUnit` _hitactor)
        (:`then`
          (if (`|EnumEquality` (`MyCharacter.Team` _asbp_basic_unit) "AI")
            (set `WeaponComponent.TargetToAttack` _asbp_basic_unit (`MyCharacter.WeaponComponent` _array_element))
            (bind _returnvalue (`AIBlueprintHelperLibrary.GetAIController` _array_element))
            (`NavigationSystem.SimpleMoveToLocation` _returnvalue (`self.K2_GetActorLocation` _asbp_basic_unit))
            (else
              (`NavigationSystem.SimpleMoveToLocation` _returnvalue _location :!label _label_2))))
        (:`CastFailed`
          (goto _label_2))))))

(event `InputAxisKey|MouseY`
  (params (AxisValue :type "Float (single-precision)"))
  ;[0.1952 1 0.08493] Camera movement
  ;;[1 1 1] pan Y
  (`/Engine/EditorBlueprintResources/StandardMacros.Gate` true :!label _label_3
    (:`Exit`
      (`self.K2_SetActorRotation` (`self.CameraPawnRef`) (`KismetMathLibrary.MakeRotator` (.roll (`self.K2_GetActorRotation` (`self.CameraPawnRef`))) (`KismetMathLibrary.FClamp` (+ (.pitch (`self.K2_GetActorRotation` (`self.CameraPawnRef`))) (* (`self.PanSensitivity`) AxisValue)) -15.0 45.0) (.yaw (`self.K2_GetActorRotation` (`self.CameraPawnRef`)))) false))))

(event `InputAction|pan`
  (params (Key :type "Key Structure"))
  ;[0.1952 1 0.08493] Camera movement
  ;;[1 1 1] pan Y
  (:`Pressed`
    (set `self.bDisableCamNav` true)
    (goto _label_3 :!via `Open`))
  (:`Released`
    (set `self.bDisableCamNav` false)
    (goto _label_3 :!via `Close`)))

(event `InputAxisKey|MouseY`
  (params (AxisValue :type "Float (single-precision)"))
  (bind _movesensitivity (`self.MovementSpeedCalculation`))
  (bind (_locationx _locationy) (`self.GetMousePosition`))
  (bind _fastmovemultiplier (`self.FastMoveMultiplier`))
  (bind _camerapawnref (`self.CameraPawnRef`))
  (bind (_x _y) (`KismetMathLibrary.BreakVector2D` (`WidgetLayoutLibrary.GetViewportSize`)))
  ;[0.1952 1 0.08493] Camera movement
  ;;[1 1 1] Screen edge movement X
  (if (`self.bDisableCamNav`)
    _
    (elif (>= (/ _locationy _y) 0.975)
      (`self.K2_SetActorTransform` (`self.CameraPawnRef`) (`self.MovementX` -1.0 _movesensitivity _fastmovemultiplier _camerapawnref) false false)
      (elif (<= (/ _locationy _y) 0.025)
        (`self.K2_SetActorTransform` (`self.CameraPawnRef`) (`self.MovementX` 1.0 _movesensitivity _fastmovemultiplier _camerapawnref) false false)))))

(event `InputAxisKey|MouseX`
  (params (AxisValue :type "Float (single-precision)"))
  (bind _movesensitivity (`self.MovementSpeedCalculation`))
  (bind _locationx (`self.GetMousePosition`))
  (bind _fastmovemultiplier (`self.FastMoveMultiplier`))
  (bind _camerapawnref (`self.CameraPawnRef`))
  (bind _x (`KismetMathLibrary.BreakVector2D` (`WidgetLayoutLibrary.GetViewportSize`)))
  ;[0.1952 1 0.08493] Camera movement
  ;;[1 1 1] Screen edge movement Y
  (if (`self.bDisableCamNav`)
    _
    (elif (>= (/ _locationx _x) 0.975)
      (`self.K2_SetActorTransform` (`self.CameraPawnRef`) (`self.MovementY` 1.0 _movesensitivity _fastmovemultiplier _camerapawnref) false false)
      (elif (<= (/ _locationx _x) 0.025)
        (`self.K2_SetActorTransform` (`self.CameraPawnRef`) (`self.MovementY` -1.0 _movesensitivity _fastmovemultiplier _camerapawnref) false false)))))

(fn `MovementSpeedCalculation`
  (returns (MoveSensitivity :type "Float (double-precision)"))
  (return (`KismetMathLibrary.FClamp` (/ (`SpringArmComponent.TargetArmLength` (`/Game/MainContent/Blueprints/BP_PlayerCameraPawn.SpringArm` (`self.CameraPawnRef`))) 50.0) 5.0 30.0)))

(fn `MoveToHitByUE4`
  (params (Hit :type "HitResult Structure (by ref)"))
  (bind (_bblockinghit _binitialoverlap _time _distance _location) (`GameplayStatics.BreakHitResult` Hit))
  (if (>= (`KismetMathLibrary.VSize` (- (`self.K2_GetActorLocation` (`self.K2_GetPawn`)) _location)) (`self.MinClickDistance`))
    (`NavigationSystem.SimpleMoveToLocation` self _location) ; Send the destination point to the character
  ))

(fn `SetSightDistance`
  (returns (SightDistance :type "Float (double-precision)"))
  (return (+ (`self.SightDistance`) (`SpringArmComponent.TargetArmLength` (`/Game/MainContent/Blueprints/BP_PlayerCameraPawn.SpringArm` (`self.CameraPawnRef`))))))

(fn `SortMyCharactersByTeam`
  (params (Characters :type "Array of MyCharacter Object Reference") (Team :type "ETeam Enum" :default "Player"))
  (returns (SortedCharacters :type "Array of MyCharacter Object Reference"))
  (locals (SortedByTeamCharacters :type "Array of MyCharacter Object Reference"))
  (bind _sortedbyteamcharacters (`local.SortedByTeamCharacters`))
  (for _array_element Characters
    (if (`|EnumEquality` (`MyCharacter.Team` _array_element) Team)
      (`KismetArrayLibrary.Array_Add` _sortedbyteamcharacters _array_element)))
  (return _sortedbyteamcharacters))

(fn `UserConstructionScript`)