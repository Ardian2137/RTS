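; HUD Blueprint that creates the WB_Hud widget and handles drag-box unit selection.
; Tick reads the selection flags on BP_MyPlayerController, anchoring the first corner at the mouse and moving the second with it.
; While selection is active, DrawHUD draws a translucent green rectangle and writes the BP_BasicUnit actors inside on the Player team back to the controller, using MyGetActorsInSelectionRectangle.
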(event `self.ReceiveDrawHUD`
  (params (SizeX :type Integer) (SizeY :type Integer))
  (bind _selectionrecx1 (`self.SelectionRecX1`))
  (bind _selectionrecy1 (`self.SelectionRecY1`))
  (if (`/Game/MainContent/Blueprints/BP_MyPlayerController.bSelectionRecActive` (stale `self.ReceiveTick` _asbp_my_player_controller))
    (`self.DrawRect` (struct :`R` 0.063832 :`G` 1.0 :`B` 0.135202 :`A` 0.514) _selectionrecx1 _selectionrecy1 (- (`self.SelectionRecX2`) _selectionrecx1) (- (`self.SelectionRecY2`) _selectionrecy1))
    (set `/Game/MainContent/Blueprints/BP_MyPlayerController.UnitsSelectedByHUD` (`self.GetSelectedActors`) (stale `self.ReceiveTick` _asbp_my_player_controller))))

(event `self.ReceiveTick`
  (params (DeltaSeconds :type "Float (single-precision)"))
  (bind (_locationx _locationy) (`PlayerController.GetMousePosition` (`GameplayStatics.GetPlayerController` 0)))
  (bind _asbp_my_player_controller (cast `/Game/MainContent/Blueprints/BP_MyPlayerController` (`GameplayStatics.GetPlayerController` 0)))
  (if (`/Game/MainContent/Blueprints/BP_MyPlayerController.bSelectionRecActive` _asbp_my_player_controller)
    (if (`/Game/MainContent/Blueprints/BP_MyPlayerController.b1stPointSet` _asbp_my_player_controller)
      (set `self.SelectionRecX1` _locationx)
      (set `self.SelectionRecY1` _locationy)
      (set `self.SelectionRecX2` _locationx)
      (set `self.SelectionRecY2` _locationy)
      (set `/Game/MainContent/Blueprints/BP_MyPlayerController.b1stPointSet` false _asbp_my_player_controller)
      (else
        (set `self.SelectionRecX2` _locationx)
        (set `self.SelectionRecY2` _locationy)))))

(event `self.ReceiveBeginPlay`
  (bind _returnvalue (`|CreateWidget` "/Game/MainContent/UI/CombatHud/WB_Hud.WB_Hud_C"))
  (`UserWidget.AddToViewport` _returnvalue 0))

(fn `GetSelectedActors`
  (returns (SelectedActors :type "Array of MyCharacter Object Reference"))
  (locals (SelectedUnits :type "Array of MyCharacter Object Reference"))
  (for _array_element (`self.MyGetActorsInSelectionRectangle` "/Game/MainContent/Blueprints/BP_BasicUnit.BP_BasicUnit_C" (`KismetMathLibrary.MakeVector2D` (`self.SelectionRecX1`) (`self.SelectionRecY1`)) (`KismetMathLibrary.MakeVector2D` (`self.SelectionRecX2`) (`self.SelectionRecY2`)))
    (bind _asbp_basic_unit (cast `/Game/MainContent/Blueprints/BP_BasicUnit` _array_element))
    (if (`|EnumEquality` (`MyCharacter.Team` _asbp_basic_unit) "Player")
      (`KismetArrayLibrary.Array_Add` (`local.SelectedUnits`) _asbp_basic_unit)))
  (return (`local.SelectedUnits`)))

(fn `UserConstructionScript`)