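; BP_GlobalFunctions is a set of shared helper functions that return the game's core objects already cast to their project Blueprint types.
; It fetches the player controller and player camera pawn at player index 0, plus the current game state.
; Each getter casts to BP_MyPlayerController, BP_PlayerCameraPawn or BP_MyGameState and returns a value only when that cast succeeds.
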(fn `GetMyGameState`
  (returns (MyGameState :type "/Game/MainContent/GameBPs/BP_MyGameState Object Reference"))
  (bind _asbp_my_game_state (cast `/Game/MainContent/GameBPs/BP_MyGameState` (`GameplayStatics.GetGameState` null)))
  (return _asbp_my_game_state))

(fn `GetMyPlayerController`
  (returns (MyPlayerController :type "/Game/MainContent/Blueprints/BP_MyPlayerController Object Reference"))
  (bind _asbp_my_player_controller (cast `/Game/MainContent/Blueprints/BP_MyPlayerController` (`GameplayStatics.GetPlayerController` null)))
  (return _asbp_my_player_controller))

(fn `GetPlayerCameraPawn`
  (returns (PlayerCameraPawnn :type "/Game/MainContent/Blueprints/BP_PlayerCameraPawn Object Reference"))
  (bind _asbp_player_camera_pawn (cast `/Game/MainContent/Blueprints/BP_PlayerCameraPawn` (`GameplayStatics.GetPlayerPawn` null)))
  (return _asbp_player_camera_pawn))